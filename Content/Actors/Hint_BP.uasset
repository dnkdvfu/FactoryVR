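; Hint actor that shows a text hint while the player's DefaultPawn is inside its overlap area.
; The construction script sets the Text component's content from the InitText variable.
; Begin and end overlap events cast the other actor to DefaultPawn and toggle the text's visibility on and off.
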(event `self.ReceiveActorBeginOverlap`
  (params (OtherActor :type "Actor Object Reference"))
  (cast `DefaultPawn` OtherActor)
  (`SceneComponent.SetVisibility` (`self.Text`) true false))

(event `self.ReceiveActorEndOverlap`
  (params (OtherActor :type "Actor Object Reference"))
  (cast `DefaultPawn` OtherActor)
  (`SceneComponent.SetVisibility` (`self.Text`) false false))

(fn `UserConstructionScript`
  (`TextRenderComponent.K2_SetText` (`self.Text`) (`self.InitText`)))