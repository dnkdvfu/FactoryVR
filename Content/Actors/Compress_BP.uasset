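; Compress_BP is a machine actor that turns resources held by its Getter_BP child actors into spawned Result actors.
; BeginPlay caches the two child getters in an array, and Tick polls whether every getter is full.
; When all are full, it calls PickUpResource on each and spawns a Result at the Aim transform inside the same loop, so once per getter.
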(event `self.ReceiveBeginPlay`
  (bind _asgetter_bp (cast `/Game/Actors/Getter_BP` (`ChildActorComponent.ChildActor` (`self.Getter_BP`))))
  (`KismetArrayLibrary.Array_Add` (`self.Getters`) _asgetter_bp)
  (bind _asgetter_bp_2 (cast `/Game/Actors/Getter_BP` (`ChildActorComponent.ChildActor` (`self.Getter_BP1`))))
  (`KismetArrayLibrary.Array_Add` (`self.Getters`) _asgetter_bp_2))

(event `self.ReceiveTick`
  (params (DeltaSeconds :type "Float (single-precision)"))
  (set `self.AllGetters` true)
  (for _array_element (`self.Getters`)
    (if (not (`/Game/Actors/Getter_BP.isFull` _array_element))
      (set `self.AllGetters` false)))
  (if (`self.AllGetters`)
    (for _array_element_2 (`self.Getters`)
      (`/Game/Actors/Getter_BP.Pick up Resource` _array_element_2)
      (`|SpawnActorFromClass` (`self.Result`) (`SceneComponent.K2_GetComponentToWorld` (`self.Aim`)) "Undefined" "MultiplyWithRoot" null null))))

(fn `UserConstructionScript`)