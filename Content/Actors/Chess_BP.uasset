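; Chess_BP is an actor that collects Resource_BP actors overlapping it and displays a tally of what it holds.
; Each overlap increments that resource type's count in the Items map, then destroys the resource.
; UpdateText rebuilds a single "name xCount" string from the map's entries and writes it to a text render.
; The construction script takes that text render from its Hint_BP child actor.
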(event `self.ReceiveActorBeginOverlap`
  (params (OtherActor :type "Actor Object Reference"))
  (bind _items (`self.Items`))
  (bind _asresource_bp (cast `/Game/Actors/Resource/Resource_BP` OtherActor))
  (bind _type (`/Game/Actors/Resource/Resource_BP.Type` _asresource_bp))
  (bind (_value _returnvalue) (`BlueprintMapLibrary.Map_Find` _items _type))
  (if _returnvalue
    (bind _result (`/Engine/EditorBlueprintResources/StandardMacros.IncrementInt` _value)
      (:`  `
        (`BlueprintMapLibrary.Map_Add` _items _type _result)))
    (else
      (`BlueprintMapLibrary.Map_Add` _items _type 1)))
  (`self.K2_DestroyActor` _asresource_bp)
  (`self.UpdateText`))

(fn `UpdateText`
  (bind _items (`self.Items`))
  (bind _returnvalue (`BlueprintMapLibrary.Map_Length` _items))
  (if (`KismetMathLibrary.Conv_IntToBool` _returnvalue)
    (bind _keys (`BlueprintMapLibrary.Map_Keys` _items))
    (bind _values (`BlueprintMapLibrary.Map_Values` _items))
    (set `self.temp` (`|FormatText` "{name} x{count}" (`|GetArrayItem` _keys) (`|GetArrayItem` _values)))
    (bind _result (`/Engine/EditorBlueprintResources/StandardMacros.DecrementInt` _returnvalue)
      (:`  `
        (for _index (range 1 (+ _result 1))
          (set `self.temp` (`|FormatText` "{Before} \n{Name} x{count}" (`self.temp`) (`|GetArrayItem` _keys _index) (`|GetArrayItem` _values _index))))
        (`TextRenderComponent.K2_SetText` (`self.TextRender`) (`self.temp`))))))

(fn `UserConstructionScript`
  (bind _ashint_bp (cast `/Game/Actors/Hint_BP` (`ChildActorComponent.ChildActor` (`self.Hint_BP`))))
  (set `self.TextRender` (`/Game/Actors/Hint_BP.Text` _ashint_bp)))