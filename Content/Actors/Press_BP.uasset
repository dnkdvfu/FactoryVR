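; Press actor that converts an overlapping actor of one class into a new actor of another class.
; On overlap, an actor whose class exactly matches From is destroyed and a To actor spawns immediately at the StaticMesh's world location.
; Cylinder1 then plays a down-and-up stroke through two timed MoveComponentTo calls sequenced by delays.
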(event `self.ReceiveBeginPlay`)

(event `self.ReceiveActorBeginOverlap`
  (params (OtherActor :type "Actor Object Reference"))
  (if (== (`self.From`) (`GameplayStatics.GetObjectClass` OtherActor))
    (`self.K2_DestroyActor` OtherActor)
    (`|SpawnActorFromClass` (`self.To`) (`KismetMathLibrary.Conv_VectorToTransform` (`SceneComponent.K2_GetComponentLocation` (`self.StaticMesh`))) "Undefined" "MultiplyWithRoot" null null)
    (`KismetSystemLibrary.MoveComponentTo` (`self.Cylinder1`) (0.0 7.5 80.0) (struct) false false 1.0)
    (`KismetSystemLibrary.Delay` 1.0)
    (`KismetSystemLibrary.MoveComponentTo` (`self.Cylinder1`) (0.0 7.5 100.0) (struct) false false 1.0)
    (`KismetSystemLibrary.Delay` 1.0)))

(fn `UserConstructionScript`)