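; Getter_BP is an actor that takes in a single resource of a required type.
; On overlap, while not full, it casts the other actor to Resource_BP, compares its Type to NeedType, and on a match destroys it and sets IsFull.
; PickUpResource clears IsFull so the getter can accept another resource.
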(event `self.ReceiveActorBeginOverlap`
  (params (OtherActor :type "Actor Object Reference"))
  (if (not (`self.isFull`))
    (bind _asresource_bp (cast `/Game/Actors/Resource/Resource_BP` OtherActor))
    (if (`KismetStringLibrary.EqualEqual_StrStr` (`/Game/Actors/Resource/Resource_BP.Type` _asresource_bp) (`self.NeedType`))
      (`self.K2_DestroyActor` OtherActor)
      (set `self.isFull` true))))

(fn `Pick up Resource`
  (set `self.isFull` false))

(fn `UserConstructionScript`)